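; BP_ResetButton is an interactable button that broadcasts a reset request for machines when the player uses it.
; Sphere overlap events set an in-range flag and toggle the helper text.
; Tick polls the E key while in range and feeds a DoOnce, which calls OnResetRequest and prints a confirmation.
; Leaving the sphere re-arms the DoOnce, limiting requests to one until the overlap ends.
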(event `self.Sphere.OnComponentBeginOverlap`
  (params (OverlappedComponent :type "PrimitiveComponent Object Reference") (OtherActor :type "Actor Object Reference") (OtherComp :type "PrimitiveComponent Object Reference") (OtherBodyIndex :type Integer) (bFromSweep :type Boolean) (SweepResult :type "HitResult Structure (by ref)"))
  (bind _output_get (set `self.Box` true))
  (`SceneComponent.SetVisibility` (`self.HelpfulText`) _output_get false))

(event `self.Sphere.OnComponentEndOverlap`
  (params (OverlappedComponent :type "PrimitiveComponent Object Reference") (OtherActor :type "Actor Object Reference") (OtherComp :type "PrimitiveComponent Object Reference") (OtherBodyIndex :type Integer))
  (set `self.Box` false)
  (`SceneComponent.SetVisibility` (`self.HelpfulText`) false false)
  (goto _label :!via `Reset`))

(event `self.ReceiveTick`
  (params (DeltaSeconds :type "Float (single-precision)"))
  (if (`self.Box`)
    (if (`PlayerController.IsInputKeyDown` (`GameplayStatics.GetPlayerController` 0) "E")
      (`/Engine/EditorBlueprintResources/StandardMacros.DoOnce` false :!label _label
        (:`Completed`
          (`self.OnResetRequest`)
          (`KismetSystemLibrary.PrintString` "Reset request received. Machines will be reset soon..."))))))

(fn `UserConstructionScript`)