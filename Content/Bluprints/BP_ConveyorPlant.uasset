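; Conveyor plant actor with a swappable mesh that can be picked up into an inventory actor.
; EnablePickup arms it and stores the inventory; Tick then polls the E key while anything overlaps its Sphere.
; Pickup attaches the plant to that inventory, hides it and deactivates its components; MakeVisible unhides and reactivates them without detaching.
; UpdateMesh picks the plant's mesh from an array, starting with the first on BeginPlay.
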(event `self.ReceiveBeginPlay`
  ; Update model
  (`self.UpdateMesh` 0))

(event `self.Sphere.OnComponentBeginOverlap`
  (params (OverlappedComponent :type "PrimitiveComponent Object Reference") (OtherActor :type "Actor Object Reference") (OtherComp :type "PrimitiveComponent Object Reference") (OtherBodyIndex :type Integer) (bFromSweep :type Boolean) (SweepResult :type "HitResult Structure (by ref)"))
  ; Collision
  (set `self.inArea` true))

(event `self.ReceiveTick`
  (params (DeltaSeconds :type "Float (single-precision)"))
  ; Pickup logic
  (if (`self.inArea`)
    (if (`self.pickupEnabled`)
      (if (`PlayerController.IsInputKeyDown` (`GameplayStatics.GetPlayerController` 0) "E")
        (set `self.pickupEnabled` false)
        (`|ExecutionSequence`
          (:`then_0`
            (`self.K2_AttachToActor` (`self.Player Inventory`) "None" "KeepRelative" "KeepRelative" "KeepRelative" false))
          (:`then_1`
            ; Hide
            (`self.SetActorHiddenInGame` true)
            (for _array_element (`self.K2_GetComponentsByClass` "/Script/Engine.ActorComponent")
              (`ActorComponent.SetActive` _array_element false false))))))))

(event `self.Sphere.OnComponentEndOverlap`
  (params (OverlappedComponent :type "PrimitiveComponent Object Reference") (OtherActor :type "Actor Object Reference") (OtherComp :type "PrimitiveComponent Object Reference") (OtherBodyIndex :type Integer))
  ; Collision
  (set `self.inArea` false))

(fn `EnablePickup`
  (params (playerInventory :type "/Game/Bluprints/BP_PlayerInventory Object Reference"))
  (set `self.pickupEnabled` true)
  (if (`KismetSystemLibrary.IsValid` playerInventory)
    (set `self.Player Inventory` playerInventory)
    (else
      (`KismetSystemLibrary.PrintString` "Null actor"))))

(fn `MakeVisible`
  (`self.SetActorHiddenInGame` false)
  (for _array_element (`self.K2_GetComponentsByClass` "/Script/Engine.ActorComponent")
    (`ActorComponent.SetActive` _array_element true false)))

(fn `UpdateMesh`
  (params (mesh :type Integer))
  (`StaticMeshComponent.SetStaticMesh` (`self.Plant`) (`|GetArrayItem` (`self.meshArray`) mesh)))

(fn `UserConstructionScript`)