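; BP_Conveyor is a conveyor Blueprint that tracks plant actors in a Slots array.
; On BeginPlay it spawns a plant at the Stage1 transform, attaches it to ConveyorPlants and stores it in the array.
; ButtonClicked records the button index; only button 0 is handled, shifting a valid plant to the next slot and clearing the old one.
; Only array entries move, and the MoveIntoNextElemnt graph is unwired.
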(event `self.ReceiveBeginPlay`
  ; Initial Plant spawn
  (bind _returnvalue (`|SpawnActorFromClass` (`self.PrefabConveyorPlant`) (`SceneComponent.GetRelativeTransform` (`self.Stage_1`)) "AlwaysSpawn" "MultiplyWithRoot" null null))
  (`self.K2_AttachToComponent` _returnvalue (`self.ConveyorPlants`) "None" "KeepRelative" "KeepRelative" "KeepRelative" false)
  (`KismetArrayLibrary.Array_Set` (`self.Slots`) (`self.spawnArrayElement`) _returnvalue))

(fn `ButtonClicked`
  (params (`Button ID` :type Integer))
  (locals (buttonIndex :type Integer) (`+1` :type Integer :default 1))
  (bind _output (`|GetArrayItem` (`self.Slots`) `Button ID`))
  ; Switch value from button
  (`|ExecutionSequence`
    (:`then_0`
      (set `local.buttonIndex` `Button ID`))
    (:`then_1`
      (switch `int` `Button ID`
        (:`0`
          ; Handle Array
          (if (`KismetSystemLibrary.IsValid` _output)
            (`KismetArrayLibrary.Array_Set` (`self.Slots`) (+ (`local.buttonIndex`) (`local.+1`)) _output)
            (`KismetArrayLibrary.Array_Set` (`self.Slots`) (`local.buttonIndex`))))))))

(fn `UserConstructionScript`)