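; BP_Button is an interactable button that signals a referenced conveyor when the player holds E nearby.
; Sphere overlap begin and end set the Caixa flag and toggle the HelpfulText prompt, without filtering which actor overlaps.
; Tick polls the E key while the flag is set and passes ButtonID to the conveyor's ButtonClicked on every frame the key is down.
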(event `self.Sphere.OnComponentBeginOverlap`
  (params (OverlappedComponent :type "PrimitiveComponent Object Reference") (OtherActor :type "Actor Object Reference") (OtherComp :type "PrimitiveComponent Object Reference") (OtherBodyIndex :type Integer) (bFromSweep :type Boolean) (SweepResult :type "HitResult Structure (by ref)"))
  (bind _output_get (set `self.caixa` true))
  (`SceneComponent.SetVisibility` (`self.HelpfulText`) _output_get false))

(event `self.Sphere.OnComponentEndOverlap`
  (params (OverlappedComponent :type "PrimitiveComponent Object Reference") (OtherActor :type "Actor Object Reference") (OtherComp :type "PrimitiveComponent Object Reference") (OtherBodyIndex :type Integer))
  (set `self.caixa` false)
  (`SceneComponent.SetVisibility` (`self.HelpfulText`) false false))

(event `self.ReceiveTick`
  (params (DeltaSeconds :type "Float (single-precision)"))
  (if (`self.caixa`)
    (if (`PlayerController.IsInputKeyDown` (`GameplayStatics.GetPlayerController` 0) "E")
      ; Button close
      (`/Game/Bluprints/BP_Conveyor.ButtonClicked` (`self.convyor`) (`self.Button ID`)))))

(fn `UserConstructionScript`)