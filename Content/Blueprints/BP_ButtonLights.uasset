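; BP_ButtonLights is an interactable button that toggles every LightActor in the level and recolors them.
; OnInteract passes each light the flipped on/off state and the next LightColor entry, wrapping the persistent index with modulo and playing a click per light.
; A sphere trigger shows and hides feedback text on overlap.
; IsInteractable always returns false, though OnInteract does not check it.
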(event `self.Sphere.OnComponentBeginOverlap`
  (params (OverlappedComponent :type "PrimitiveComponent Object Reference") (OtherActor :type "Actor Object Reference") (OtherComp :type "PrimitiveComponent Object Reference") (OtherBodyIndex :type Integer) (bFromSweep :type Boolean) (SweepResult :type "HitResult Structure (by ref)"))
  ; Shows a text feedback when the player approaches the trigger
  (`SceneComponent.SetVisibility` (`self.feedbackText`) true false))

(event `self.Sphere.OnComponentEndOverlap`
  (params (OverlappedComponent :type "PrimitiveComponent Object Reference") (OtherActor :type "Actor Object Reference") (OtherComp :type "PrimitiveComponent Object Reference") (OtherBodyIndex :type Integer))
  ; Shows a text feedback when the player approaches the trigger
  (`SceneComponent.SetVisibility` (`self.feedbackText`) false false))

(event `/Game/Blueprints/Interfaces/BPI_Interactible.OnInteract`
  (params (interactingCharacter :type "Character Object Reference"))
  (bind _lightcolor (`self.lightColor`))
  ; Updates all the lights of the game
  (bind _outactors (`GameplayStatics.GetAllActorsOfClass` (`self.lightActor`)))
  (for _array_element _outactors
    (`/Game/Blueprints/BP_Light.UpdateLight` _array_element (not (`self.lightEnabled`)) (`|GetArrayItem` _lightcolor (`self.nextColorIndex`)))
    (set `self.nextColorIndex` (mod (+ (`self.nextColorIndex`) 1) (`KismetArrayLibrary.Array_Length` _lightcolor)))
    (`GameplayStatics.PlaySound2D` (`self.clickSound`) 1.0 1.0 0.0 null null))
  (set `self.lightEnabled` (not (`self.lightEnabled`))))

(fn `IsInteractable`
  (returns (interactable :type Boolean))
  (return false))

(fn `UserConstructionScript`)