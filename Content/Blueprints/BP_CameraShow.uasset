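; BP_CameraShow plays a timed camera showcase at level start, then switches back to the player's default camera.
; BeginPlay disables player input, then retries every two seconds until the BP_ThirdPersonCharacter cast succeeds.
; It calls the character's UpdatePlayerCamera for two views and the default, spaced by WaitTime, which also sets blend duration.
; Input is not re-enabled here, and an unconnected duplicate sequence never runs.
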(event `self.ReceiveBeginPlay`
  (bind _returnvalue (`GameplayStatics.GetPlayerController` 0))
  (bind _waittime (`self.waitTime`))
  (`self.DisableInput` _returnvalue _returnvalue)
  (`KismetSystemLibrary.Delay` 2.0 :!label _label)
  (bind _asbp_third_person_character (cast `/Game/Blueprints/BP_ThirdPersonCharacter` (`GameplayStatics.GetPlayerCharacter` 0))
    (:`then`
      (`/Game/Blueprints/BP_ThirdPersonCharacter.UpdatePlayerCamera` _asbp_third_person_character false "/Script/Engine.CameraActor" _waittime 0)
      (`KismetSystemLibrary.Delay` _waittime)
      (`/Game/Blueprints/BP_ThirdPersonCharacter.UpdatePlayerCamera` _asbp_third_person_character false "/Script/Engine.CameraActor" _waittime 1)
      (`KismetSystemLibrary.Delay` _waittime)
      (`/Game/Blueprints/BP_ThirdPersonCharacter.UpdatePlayerCamera` _asbp_third_person_character true "/Script/Engine.CameraActor" _waittime 0))
    (:`CastFailed`
      (goto _label))))

(fn `UserConstructionScript`)