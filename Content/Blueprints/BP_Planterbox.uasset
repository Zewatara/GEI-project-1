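; BP_Planterbox is a five-slot planter that takes plants from the player's inventory and broadcasts a looping growth tick.
; Overlapping a slot's collider runs PlantAttempt, which takes the first actor attached to PlayerInventory if that slot is free.
; The BP_ConveyorPlant is made visible, enabled, stored in PlantSlots and snapped onto the collider.
; A reset request from BPResetButton destroys all planted actors.
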(event `self.ReceiveBeginPlay`
  ; Prepare global event
  (`KismetSystemLibrary.K2_SetTimerDelegate` (delegate `call global`) (`self.growthTime`) true)
  ; Bind to reset global
  (add `/Game/Blueprints/BP_ResetButton.OnResetRequest` (`self.BP_ResetButton`) (delegate `CallResetQuest`)))

(event `self.col1.OnComponentBeginOverlap`
  (params (OverlappedComponent :type "PrimitiveComponent Object Reference") (OtherActor :type "Actor Object Reference") (OtherComp :type "PrimitiveComponent Object Reference") (OtherBodyIndex :type Integer) (bFromSweep :type Boolean) (SweepResult :type "HitResult Structure (by ref)"))
  ; Handle collisions
  (`self.PlantAttempt` (`self.playerInventory`) 0 (`self.col1`)))

(event `CallResetQuest`
  ; Bind to reset global
  (`self.ResetMachine`))

(event `call global`
  ; Prepare global event
  (`self.OnGrowTick`))

(event `self.col2.OnComponentBeginOverlap`
  (params (OverlappedComponent :type "PrimitiveComponent Object Reference") (OtherActor :type "Actor Object Reference") (OtherComp :type "PrimitiveComponent Object Reference") (OtherBodyIndex :type Integer) (bFromSweep :type Boolean) (SweepResult :type "HitResult Structure (by ref)"))
  ; Handle collisions
  (`self.PlantAttempt` (`self.playerInventory`) 1 (`self.col2`)))

(event `self.col3.OnComponentBeginOverlap`
  (params (OverlappedComponent :type "PrimitiveComponent Object Reference") (OtherActor :type "Actor Object Reference") (OtherComp :type "PrimitiveComponent Object Reference") (OtherBodyIndex :type Integer) (bFromSweep :type Boolean) (SweepResult :type "HitResult Structure (by ref)"))
  ; Handle collisions
  (`self.PlantAttempt` (`self.playerInventory`) 2 (`self.col3`)))

(event `self.col4.OnComponentBeginOverlap`
  (params (OverlappedComponent :type "PrimitiveComponent Object Reference") (OtherActor :type "Actor Object Reference") (OtherComp :type "PrimitiveComponent Object Reference") (OtherBodyIndex :type Integer) (bFromSweep :type Boolean) (SweepResult :type "HitResult Structure (by ref)"))
  ; Handle collisions
  (`self.PlantAttempt` (`self.playerInventory`) 3 (`self.col4`)))

(event `self.col5.OnComponentBeginOverlap`
  (params (OverlappedComponent :type "PrimitiveComponent Object Reference") (OtherActor :type "Actor Object Reference") (OtherComp :type "PrimitiveComponent Object Reference") (OtherBodyIndex :type Integer) (bFromSweep :type Boolean) (SweepResult :type "HitResult Structure (by ref)"))
  ; Handle collisions
  (`self.PlantAttempt` (`self.playerInventory`) 4 (`self.col5`)))

(fn `PlantAttempt`
  (params (playerInventory :type "/Game/Blueprints/BP_PlayerInventory Object Reference") (plantSlot :type Integer) (boxCollider :type "BoxComponent Object Reference"))
  (locals (colliderPlantBox :type "BoxComponent Object Reference") (selectedSlot :type Integer))
  (bind _outactors (`self.GetAttachedActors` playerInventory true false))
  (bind _output (`|GetArrayItem` _outactors))
  (`|ExecutionSequence`
    (:`then_0`
      ; Update local variables
      (set `local.colliderPlantBox` boxCollider)
      (set `local.selectedSlot` plantSlot))
    (:`then_1`
      ; Check slot
      (if (>= (`KismetArrayLibrary.Array_Length` _outactors) 1)
        (if (not (`KismetSystemLibrary.IsValid` (`|GetArrayItem` (`self.plantSlots`) plantSlot)))
          (`|ExecutionSequence`
            (:`then_0`
              ; Handle visibillity and relative location
              (bind _asbp_conveyor_plant (cast `/Game/Blueprints/BP_ConveyorPlant` _output))
              (`/Game/Blueprints/BP_ConveyorPlant.ChangeVisible` _asbp_conveyor_plant true)
              (`/Game/Blueprints/BP_ConveyorPlant.UpdateMesh` _asbp_conveyor_plant 3)
              ;; Makes sure the actor ends up in the correct place.
              (`self.K2_SetActorRelativeLocation` _asbp_conveyor_plant (0.0 0.0 0.0) false true)
              (`/Game/Blueprints/BP_ConveyorPlant.EnablePlant` _asbp_conveyor_plant)
              ; Update array
              (`KismetArrayLibrary.Array_Set` (`self.plantSlots`) (`local.selectedSlot`) _asbp_conveyor_plant))
            (:`then_1`
              ; Attaches the plant to the new splot
              (`self.K2_AttachToComponent` _output (`local.colliderPlantBox`) "None" "KeepWorld" "KeepWorld" "KeepWorld" false)
              ; test
              (`SceneComponent.ResetRelativeTransform` (`Actor.RootComponent` _asbp_conveyor_plant)))))))))

(fn `ResetMachine`
  (for _array_element (`self.plantSlots`)
    (if (`KismetSystemLibrary.IsValid` _array_element)
      (`self.K2_DestroyActor` _array_element)))
  (`KismetSystemLibrary.PrintString` "Planter box as has cleared!"))

(fn `UserConstructionScript`)