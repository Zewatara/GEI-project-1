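; BP_ResetButton is an interactable button that requests a game state reset, apparently for machines.
; A sphere trigger shows and hides a feedback text on begin and end overlap, without filtering the overlapping actor.
; OnInteract, noted as called from the player character, fires the global OnResetRequest event, prints a confirmation and plays a click sound.
; IsInteractable always returns false.
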(event `self.Sphere.OnComponentBeginOverlap`
  (params (OverlappedComponent :type "PrimitiveComponent Object Reference") (OtherActor :type "Actor Object Reference") (OtherComp :type "PrimitiveComponent Object Reference") (OtherBodyIndex :type Integer) (bFromSweep :type Boolean) (SweepResult :type "HitResult Structure (by ref)"))
  ; Shows a text feedback when the player approaches the trigger
  (`SceneComponent.SetVisibility` (`self.feedbackText`) true false))

(event `self.Sphere.OnComponentEndOverlap`
  (params (OverlappedComponent :type "PrimitiveComponent Object Reference") (OtherActor :type "Actor Object Reference") (OtherComp :type "PrimitiveComponent Object Reference") (OtherBodyIndex :type Integer))
  ; Shows a text feedback when the player approaches the trigger
  (`SceneComponent.SetVisibility` (`self.feedbackText`) false false))

(event `/Game/Blueprints/Interfaces/BPI_Interactible.OnInteract`
  (params (interactingCharacter :type "Character Object Reference"))
  ; Cast global event to reset the game state. Event is called from the player character
  (`self.OnResetRequest`)
  (`KismetSystemLibrary.PrintString` "Reset request received. Machines will be reset soon...")
  (`GameplayStatics.PlaySoundAtLocation` (`self.clickSound`) (`SceneComponent.K2_GetComponentLocation` (`self.DefaultSceneRoot`)) (struct) 1.0 1.0 0.0 null null null null))

(fn `IsInteractable`
  (returns (interactable :type Boolean))
  (return false))

(fn `UserConstructionScript`)