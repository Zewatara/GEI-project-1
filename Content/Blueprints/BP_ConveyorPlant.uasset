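; BP_ConveyorPlant is a plant actor that grows through visual stages once planted and can be stowed in the player's inventory.
; It binds to the grow tick of the first BPPlantBox found, counting ticks up to GrowTime before swapping its static mesh from an array.
; Interaction disables physics, attaches it to the inventory, hides it and resets the player camera, though IsInteractable always returns false.
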(event `grow`
  ; Binds the global grow event to the growing behaviour of the plant. It only happens if it is currently planted.
  (if (`self.isplanted`)
    ; Handles the growing behaviour of plants based on plant type. Updates mesh to represent the stage corretly
    (if (== (`self.currentgrowth`) (`self.growTime`))
      (`|ExecutionSequence`
        (:`then_0`
          (switch `int` (`self.growthstage`)
            (:`0`
              (`self.UpdateMesh` 4)
              (set `self.growthstage` 1))
            (:`1`
              (`self.UpdateMesh` 5)
              (set `self.growthstage` 2))))
        (:`then_1`
          (set `self.currentgrowth` 0)))
      (else
        (set `self.currentgrowth` (+ (`self.currentgrowth`) 1))))))

(event `self.ReceiveBeginPlay`
  (`|ExecutionSequence`
    (:`then_0`
      ; Updates the mesh based on the first stage of the plant type.
      (`self.UpdateMesh` 0))
    (:`then_1`
      ; Binds the global grow event to the growing behaviour of the plant. It only happens if it is currently planted.
      (bind _outactors (`GameplayStatics.GetAllActorsOfClass` (`self.BP_PlantBox`)))
      (add `/Game/Blueprints/BP_Planterbox.OnGrowTick` (`|GetArrayItem` _outactors) (delegate `grow`)))))

(event `/Game/Blueprints/Interfaces/BPI_Interactible.OnInteract`
  (params (interactingCharacter :type "Character Object Reference"))
  ; Player Interaction
  (`|ExecutionSequence`
    (:`then_0`
      ;; Disable physics and move into inventory
      (`PrimitiveComponent.SetSimulatePhysics` (`self.Plant`) false)
      (`self.K2_AttachToActor` (`self.Player Inventory`) "None" "KeepWorld" "KeepWorld" "KeepWorld" false)
      ;; Sanity check
      (`self.K2_SetActorLocation` (0.0 0.0 0.0) false true)
      (`self.K2_SetActorRelativeLocation` (0.0 0.0 0.0) false true))
    (:`then_1`
      (`self.ChangeVisible` false))
    (:`then_2`
      ;; Update player camera
      (bind _asbp_third_person_character (cast `/Game/Blueprints/BP_ThirdPersonCharacter` (`GameplayStatics.GetPlayerCharacter` 0)))
      (`/Game/Blueprints/BP_ThirdPersonCharacter.UpdatePlayerCamera` _asbp_third_person_character true null 4.0))))

(fn `ChangeVisible`
  (params (visible :type Boolean))
  (for _array_element (`self.K2_GetComponentsByClass` "/Script/Engine.ActorComponent")
    (`ActorComponent.SetActive` _array_element visible false))
  (`self.SetActorHiddenInGame` (not visible)))

(fn `EnablePickup`
  (params (playerInventory :type "/Game/Blueprints/BP_PlayerInventory Object Reference"))
  (set `self.pickupEnabled` true)
  (if (`KismetSystemLibrary.IsValid` playerInventory)
    (set `self.Player Inventory` playerInventory)))

(fn `EnablePlant`
  (set `self.isplanted` true))

(fn `IsInteractable`
  (returns (interactable :type Boolean))
  (return false))

(fn `UpdateMesh`
  (params (mesh :type Integer))
  (`StaticMeshComponent.SetStaticMesh` (`self.Plant`) (`|GetArrayItem` (`self.meshArray`) mesh)))

(fn `UserConstructionScript`)